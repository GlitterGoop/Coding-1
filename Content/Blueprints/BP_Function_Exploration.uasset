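; BP_Function_Exploration is a Blueprint exercise in functions that prints debug messages on BeginPlay.
; A custom Say event prints randomly colored text, which CountToNumber calls in a loop with growing durations.
; Each entry in Names prints in a color from GetColorByNameLength: black when short, white when long.
; Middle lengths use NewFunction's squared offset divided by range, yielding equal RGB values above one rather than normalized gray.
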(event Custom|Say
  (params (InString :type String) (Duration :type Float%20%28single-precision%29))
  (Development|PrintString InString true true (Utilities|Struct|MakeLinearColor (Math|Random|RandomFloat) (Math|Random|RandomFloat) (Math|Random|RandomFloat) 1.0) Duration))

(event EventBeginPlay
  (Development|PrintString "We exploring functions today" true true "(R=0.000000,G=0.660000,B=1.000000,A=1.000000)" 8.0)
  (CallFunction|Say "What's up" 5.0)
  (CallFunction|CounttoNumber 10)
  (for _array_element (Variables|Default|GetNames)
    (bind _outputcolor (CallFunction|GetColorbyNameLength _array_element))
    (Development|PrintString _array_element true true _outputcolor)))

(fn ConstructionScript)

(fn CounttoNumber
  (params (Number :type Integer))
  (for _index (range 0 Number)
    (CallFunction|Say (Utilities|String|ToString(Integer) _index) (+ (* _index 0.1) 5.0)))
  (return))

(fn GetColorbyNameLength
  (params (input :type String))
  (bind _returnvalue (Utilities|String|Len input))
  (bind _returnvalue_2 (Math|Conversions|ToFloat(Integer) _returnvalue))
  (bind _returnvalue_3 (CallFunction|NewFunction 0.0 1e+01 _returnvalue_2))
  (if (<= _returnvalue 5)
    (LocalVariables|Setoutput%20color (Utilities|Struct|MakeLinearColor 0.0 0.0 0.0 1.0))
    (elif (>= _returnvalue 10)
      (LocalVariables|Setoutput%20color (Utilities|Struct|MakeLinearColor 1.0 1.0 1.0 1.0))
      (else
        (LocalVariables|Setoutput%20color (Utilities|Struct|MakeLinearColor _returnvalue_3 _returnvalue_3 _returnvalue_3 1.0)))))
  (return (LocalVariables|Getoutput%20color)))

(fn NewFunction
  (params (min :type Float%20%28double-precision%29) (max :type Float%20%28double-precision%29) (input :type Float%20%28double-precision%29))
  (bind _returnvalue (- input min))
  (return (* _returnvalue (/ _returnvalue (- max min)))))