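; BP_CoolBox is a box actor that endlessly spawns BP_Key actors above itself.
; On BeginPlay it stores a spawn point above its Cube component and prints debug messages with its name and that position.
; It then loops through a Delay node, each pass spawning a key and playing a powerup sound at slightly randomized pitch, spaced by SpawnDelay.
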(event EventBeginPlay
  (Variables|Default|SetKey%20Spawn%20Position (+ (Transformation|GetWorldLocation (Variables|Default|GetCube)) "0.000000,0.000000,200.000000"))
  (Development|PrintString (Utilities|String|Append (Utilities|GetDisplayName self) " exists!") true true "(R=0.000000,G=0.660000,B=1.000000,A=1.000000)" 1e+01)
  (Development|PrintString (Utilities|String|ToString(Vector) (Variables|Default|GetKey%20Spawn%20Position)) true true "(R=0.289086,G=1.000000,B=0.261015,A=1.000000)" 1e+01)
  (Development|PrintString (Utilities|String|ToString(Vector) (Variables|Default|GetKey%20Spawn%20Position)) true true "(R=1.000000,G=0.177083,B=0.177083,A=1.000000)")
  (Game|SpawnActorfromClass "/Game/Blueprints/BP_Key.BP_Key_C" (Math|Transform|MakeTransform (Variables|Default|GetKey%20Spawn%20Position) "0, 0, 0" "1.000000,1.000000,1.000000") "Undefined" "MultiplyWithRoot" 0 0 :!label _label)
  (Audio|SpawnSoundatLocation "/Game/Audio/Powerup3_Cue.Powerup3_Cue" (Transformation|GetWorldLocation (Variables|Default|GetDefaultSceneRoot)) "0, 0, 0" 1.0 (Math|Random|RandomFloatinRange 0.9 1.1) 0.0 0 0)
  (Utilities|FlowControl|Delay (Variables|Default|GetSpawn%20Delay))
  (goto _label))

(fn ConstructionScript)