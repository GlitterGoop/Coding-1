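; BP_ItemTest is a test item with a random name, an elemental type and elemental damage logic.
; On BeginPlay it runs Constructor to pick a name from a hardcoded list, then prints the name and its damage against an Air victim.
; GetDamage doubles base damage when the item's element sits two steps from the victim's in the four-value cycle, using modulo arithmetic on the enum.
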(event EventBeginPlay
  (CallFunction|Constructor)
  (Development|PrintString (Utilities|String|Append "My name is " (Variables|Default|GetName)))
  (bind _damage (CallFunction|GetDamage "NewEnumerator2"))
  (Development|PrintString (Utilities|String|Append "we are " (Utilities|String|EnumtoString (Variables|Default|GetElementalType)) ", victim is air, damage =" (Utilities|String|ToString(Integer) _damage)) true true "(R=1.000000,G=0.131000,B=0.214699,A=1.000000)" 5.0))

(fn ConstructionScript)

(fn Constructor
  (bind _returnvalue (Utilities|String|MakeLiteralString "Earl"))
  (bind _returnvalue_2 (Utilities|String|MakeLiteralString "Brian"))
  (bind _returnvalue_3 (Utilities|String|MakeLiteralString "Bodie"))
  (bind _returnvalue_4 (Utilities|String|MakeLiteralString "Larry"))
  (bind _returnvalue_5 (Utilities|String|MakeLiteralString "Gorlog"))
  (bind _array (Utilities|Array|MakeArray _returnvalue_2 _returnvalue_3 _returnvalue_4 _returnvalue_5 _returnvalue))
  (if true
    (Utilities|Array|Shuffle _array)
    (Variables|Default|SetName (Utilities|Array|Get(acopy) _array (Math|Random|RandomIntegerinRange 0 (- (Utilities|Array|Length _array) 1))))))

(fn GetDamage
  (params (Victim%20ElementalType :type ElementalType%20Enum :default "NewEnumerator0"))
  (LocalVariables|SetReturn%20Damage (Variables|Default|GetDamage))
  (if (== (Class|KismetMathLibrary|PercentByteByte (+ Victim%20ElementalType 2) 4) (Math|Conversions|ToInteger(Byte) (Variables|Default|GetElementalType)))
    (LocalVariables|SetReturn%20Damage (* (Variables|Default|GetDamage) 2)))
  (return (LocalVariables|GetReturn%20Damage)))