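; BP_EnemySpawner is a manager actor that populates the level with enemies and respawns them once all are gone.
; On BeginPlay it gathers every BP_EnemySpawnLocation, prints the count for debugging, and spawns BP_Enemy at each location with roughly an 80% chance.
; A self-recursive EnemyCountCheck event polls every two seconds and triggers another spawn pass whenever no BP_Enemy actors remain.
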(event Custom|Spawn%20Enemies
  (for _array_element (stale EventBeginPlay _outactors)
    (if (> (Math|Random|RandomFloat) 0.2)
      (Game|SpawnActorfromClass "/Game/Blueprints/BP_Enemy.BP_Enemy_C" (Transformation|GetActorTransform _array_element) "Undefined" "MultiplyWithRoot" 0 0))))

(event Custom|Enemy%20Count%20Check
  (bind _outactors (Actor|GetAllActorsOfClass "/Game/Blueprints/BP_Enemy.BP_Enemy_C"))
  (if (> (Utilities|Array|Length _outactors) 0) ; If no enemies, spawn more
    _
    (else
      (CallFunction|SpawnEnemies)))
  (Utilities|FlowControl|Delay 2.0)
  (CallFunction|EnemyCountCheck))

(event EventBeginPlay
  (bind _outactors (Actor|GetAllActorsOfClass "/Game/Blueprints/BP_EnemySpawnLocation.BP_EnemySpawnLocation_C"))
  (Development|PrintString (Utilities|String|Append "There are " (Utilities|String|ToString(Integer) (Utilities|Array|Length _outactors)) " spawners") true true "(R=0.107849,G=0.000000,B=1.000000,A=1.000000)" 1e+01)
  (CallFunction|SpawnEnemies)
  (CallFunction|EnemyCountCheck))

(fn ConstructionScript)