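; BP_ActorTest is a test actor that gives itself a random name in its construction script.
; Behind an always-true branch, it shuffles a literal array of candidate names, then stores a randomly indexed entry in the Name variable.
; BeginPlay, overlap and Tick are disabled placeholders, NewFunction is empty, and a Name comparison is left unused.
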(event EventBeginPlay)

(event Collision|EventActorBeginOverlap
  (params (OtherActor :type Actor%20Object%20Reference)))

(event EventTick
  (params (DeltaSeconds :type Float%20%28single-precision%29)))

(fn ConstructionScript
  (bind _returnvalue (Utilities|String|MakeLiteralString "Earl"))
  (bind _returnvalue_2 (Utilities|String|MakeLiteralString "Brian"))
  (bind _returnvalue_3 (Utilities|String|MakeLiteralString "Bodie"))
  (bind _returnvalue_4 (Utilities|String|MakeLiteralString "Larry"))
  (bind _returnvalue_5 (Utilities|String|MakeLiteralString "Gorlog"))
  (bind _array (Utilities|Array|MakeArray _returnvalue_2 _returnvalue_3 _returnvalue_4 _returnvalue_5 _returnvalue))
  (if true
    (Utilities|Array|Shuffle _array)
    (Variables|Default|SetName (Utilities|Array|Get(acopy) _array (Math|Random|RandomIntegerinRange 0 (- (Utilities|Array|Length _array) 1))))))

(fn NewFunction)